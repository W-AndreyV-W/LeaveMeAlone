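; PC_LeaveMeAlone is a player controller that handles opening the pause menu.
; When Pause is pressed while not already paused, it sets OnPause, pauses the game, shows a new WBP_Pause widget and switches to UI-only input with the mouse cursor.
; It then calls OffFire on the CH_Player pawn's WeaponComponent.
; The controller itself has no unpause logic.
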(event `InputAction|Pause`
  (params (Key :type "Key Structure"))
  ;[1 1 1] Game pause.
  (:`Pressed`
    (if (not (`self.OnPause`))
      (`|ExecutionSequence`
        (:`then_0`
          (bind _output_get (set `self.OnPause` true))
          (`GameplayStatics.SetGamePaused` _output_get)
          (bind _returnvalue (`|GenericCreateObject` "/Game/LeaveMeAlone/Widgets/UI/WBP_Pause.WBP_Pause_C"))
          (bind _output_get_2 (set `self.PauseWidget` _returnvalue))
          (`UserWidget.AddToViewport` _output_get_2 0)
          (`WidgetBlueprintLibrary.SetInputMode_UIOnlyEx` self _output_get_2)
          (set `self.bShowMouseCursor` true))
        (:`then_1`
          (bind _asch_player (cast `/Game/LeaveMeAlone/Core/Characters/CH_Player` (`GameplayStatics.GetPlayerPawn` 0)))
          (`LMAWeaponComponent.OffFire` (`LMADefaultCharacter.WeaponComponent` _asch_player)))))))

(fn `UserConstructionScript`)