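; Game mode for the last level of LeaveMeAlone that ends the game when time runs out.
; EventTimeOver saves the max score from the game instance, then creates a WBP_GameOver widget showing the zombie count and time-over text.
; It resets the stored score to zero, adds the widget to the viewport, switches input to UI only and shows the mouse cursor.
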(event `self.EventTimeOver`
  (bind _returnvalue (`GameplayStatics.GetPlayerController` 0))
  (bind _as_gi_game_instance (`self.As GI Game Instance`))
  (bind _as_gi_game_instance_2 (`self.As GI Game Instance`))
  ;[1 1 1] Completion of the game by timer.
  (`/Engine/EditorBlueprintResources/StandardMacros.IsValid` _as_gi_game_instance_2
    (:`Is Valid`
      (`self.SaveGameMaxScore` (`LMAInstance.Score` _as_gi_game_instance_2))
      (bind _returnvalue_2 (`|CreateWidget` "/Game/LeaveMeAlone/Widgets/UI/WBP_GameOver.WBP_GameOver_C"))
      (bind _output_get (set `self.TimeOver` _returnvalue_2))
      (`/Game/LeaveMeAlone/Widgets/UI/WBP_GameOver.OnNumberZombie` _output_get (`LMAInstance.Score` _as_gi_game_instance))
      (set `LMAInstance.Score` 0 _as_gi_game_instance)
      (`/Game/LeaveMeAlone/Widgets/UI/WBP_GameOver.OnTextTimeOver` _output_get (`self.TimeOverText`))
      (`UserWidget.AddToViewport` _output_get 0)
      (`WidgetBlueprintLibrary.SetInputMode_UIOnlyEx` _returnvalue _output_get)
      (bind _aspc_leave_me_alone (cast `/Game/LeaveMeAlone/Core/Controller/PC_LeaveMeAlone` _returnvalue))
      (set `PlayerController.bShowMouseCursor` true _aspc_leave_me_alone))))

(fn `UserConstructionScript`
  (`parent.UserConstructionScript`))